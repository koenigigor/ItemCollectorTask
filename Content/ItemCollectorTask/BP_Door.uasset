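; Networked double sliding door that opens when interacted with and closes automatically after a delay.
; Interact runs only on authority, setting a replicated State of open flag plus server timestamp, then resetting it after the open and timeout period.
; OnRep_State plays or reverses a timeline sliding both panels apart, scaling play rate by replication delay so all players, including late joiners, finish the motion together.
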(event `OpenDoor_Server`
  (if (not (`.bOpen_1_C8857E534E7176A9064213892402F72F` (break `/Game/ItemCollectorTask/Structures/ST_OpenDoorTimestamp` (`self.State`))))
    ;[0.1562 0.1562 0.1562 0.5] Open door (by RepNotify)
    (set `self.State` (make `/Game/ItemCollectorTask/Structures/ST_OpenDoorTimestamp` true (`GameStateBase.GetServerWorldTimeSeconds` (`GameplayStatics.GetGameState`))))
    (`KismetSystemLibrary.Delay` (+ (`self.OpenDuration`) (`self.CloseTimeout`)))
    ;[0.1562 0.1562 0.1562 0.5] CloseDoor (by RepNotify)
    (set `self.State` (make `/Game/ItemCollectorTask/Structures/ST_OpenDoorTimestamp` false (`GameStateBase.GetServerWorldTimeSeconds` (`GameplayStatics.GetGameState`))))))

(event `OpenDoor_Local`
  ;[0.1562 0.1562 0.1562 0.5] Set play rate adjusted by replication delay
  ; (for all players finish open door in same time)
  ; (include connected in process players who not receive multicast RPC)
  (`TimelineComponent.SetPlayRate` (`self.TL_OpenDoor`) (/ 1.0 (- (`self.OpenDuration`) (- (`GameStateBase.GetServerWorldTimeSeconds` (`GameplayStatics.GetGameState`)) (`.StartActionTimetamp_4_BA3A0E4743E72C7083C8FCA648FFC6E5` (break `/Game/ItemCollectorTask/Structures/ST_OpenDoorTimestamp` (`self.State`)))))))
  (if (`.bOpen_1_C8857E534E7176A9064213892402F72F` (break `/Game/ItemCollectorTask/Structures/ST_OpenDoorTimestamp` (`self.State`)))
    (bind (_direction _alpha) (`Timeline|TL_OpenDoor` :!label _label)
      (:`Update`
        (bind _returnvalue (* (`self.OpenHalfLength`) _alpha))
        (`SceneComponent.K2_SetRelativeLocation` (`self.Right`) (`KismetMathLibrary.MakeVector` _returnvalue (.y (`SceneComponent.RelativeLocation` (`self.Right`))) (.z (`SceneComponent.RelativeLocation` (`self.Right`)))) false false)
        (`SceneComponent.K2_SetRelativeLocation` (`self.Left`) (`KismetMathLibrary.MakeVector` (* _returnvalue -1.0) (.y (`SceneComponent.RelativeLocation` (`self.Left`))) (.z (`SceneComponent.RelativeLocation` (`self.Left`)))) false false)))
    (else
      (goto _label :!via `Reverse`))))

(fn `Interact`
  (params (Pawn :type "Pawn Object Reference"))
  (returns (ReturnValue :type Boolean))
  (`/Engine/EditorBlueprintResources/ActorMacros.Switch Has Authority`
    (:`Authority`
      (`self.OpenDoor_Server`)
      (return true))
    (:`Remote`
      (return false))))

(fn `OnRep_State`
  (`self.OpenDoor_Local`))

(fn `UserConstructionScript`)