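; Teleporter actor that moves any overlapping Character to a linked destination, TeleportDestanation, using the transform of its ExitDirection component.
; On overlap, only the authority performs the teleport to that component's world location and rotation.
; Both authority and remote sides then set the Character's controller rotation to the exit rotation, when a valid controller exists, so control rotation matches the exit.
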(event `self.ReceiveActorBeginOverlap`
  (params (OtherActor :type "Actor Object Reference"))
  (bind _returnvalue (`Pawn.GetController` (`self.Overlapping Pawn`)))
  (bind _exitdirection (`/Game/ItemCollectorTask/BP_Teleport.ExitDirection` (`self.TeleportDestanation`)))
  (bind _ascharacter (cast `Character` OtherActor))
  (set `self.Overlapping Pawn` _ascharacter)
  (`self.TeleportDestanation`
    (:`then`
      (`/Engine/EditorBlueprintResources/ActorMacros.Switch Has Authority`
        (:`Authority`
          (`|ExecutionSequence`
            (:`then_0`
              (`self.K2_TeleportTo` (`self.Overlapping Pawn`) (`SceneComponent.K2_GetComponentLocation` _exitdirection) (`SceneComponent.K2_GetComponentRotation` _exitdirection)))
            (:`then_1`
              (`/Engine/EditorBlueprintResources/StandardMacros.IsValid` _returnvalue :!label _label
                (:`Is Valid`
                  (`Controller.SetControlRotation` _returnvalue (`SceneComponent.K2_GetComponentRotation` (`/Game/ItemCollectorTask/BP_Teleport.ExitDirection` (`self.TeleportDestanation`)))))))))
        (:`Remote`
          (goto _label))))
    (:`else`)))

(fn `UserConstructionScript`)