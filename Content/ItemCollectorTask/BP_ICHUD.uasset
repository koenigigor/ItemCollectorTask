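; BP_ICHUD is the HUD Blueprint for the Item Collector task, creating the match UI and the end-of-match screen.
; On BeginPlay it adds the W_ICHud widget to the viewport and binds to the ICGameState match-end event.
; When the match ends, it shows W_Winner with the winner passed in, or W_LoseByTime if no valid winner exists.
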(event `self.ReceiveBeginPlay`
  (bind _returnvalue (`|CreateWidget` "/Game/ItemCollectorTask/UI/W_ICHud.W_ICHud_C" (`self.PlayerOwner`)))
  (`UserWidget.AddToViewport` _returnvalue 0)
  (bind _asicgame_state (cast `ICGameState` (`GameplayStatics.GetGameState`)))
  (add `ICGameState.OnMatchEnd` _asicgame_state (`|CreateDelegate` :!event `OnMatchEnd`)))

(event `OnMatchEnd`
  (params (Winner :type "PlayerState Object Reference"))
  (`/Engine/EditorBlueprintResources/StandardMacros.IsValid` Winner
    (:`Is Valid`
      (bind _returnvalue (`|CreateWidget` "/Game/ItemCollectorTask/UI/W_Winner.W_Winner_C" (`self.PlayerOwner`) Winner))
      (`UserWidget.AddToViewport` _returnvalue 1))
    (:`Is Not Valid`
      (bind _returnvalue_2 (`|CreateWidget` "/Game/ItemCollectorTask/UI/W_LoseByTime.W_LoseByTime_C" (`self.PlayerOwner`)))
      (`UserWidget.AddToViewport` _returnvalue_2 1))))

(fn `UserConstructionScript`)